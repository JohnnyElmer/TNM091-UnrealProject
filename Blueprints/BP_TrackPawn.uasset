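; BP_TrackPawn is a pawn that rides the level's track spline as a timed camera ride, then advances to the next level.
; On BeginPlay it fades in, finds the first BP_Track and starts a timeline sized to TotalTime.
; The timeline samples the spline by normalized time, setting actor location and camera world rotation.
; On finish it fades to black, increments the GameInstance's LevelIndex, and opens the selected level or quits after the last.
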(event Custom|Move%20Along%20Track
  (bind _bp_track (Variables|Default|GetBP_Track))
  (bind _spline (Variables|/Game/Blueprints/BP_Track.BP_Track_C|GetSpline _bp_track))
  (Timeline|Timeline_0 PlayFromStart
    (:Update
      (Transformation|SetActorLocation (Spline|GetLocationatTime _spline (/ (Components|Timeline|GetPlaybackPosition (Variables|Default|GetTimeline_0)) (Variables|Default|GetTotal%20Time)) "World" false) false false)
      (Transformation|SetWorldRotation (Variables|Default|GetCamera) (Class|SplineComponent|GetRotationatTime _spline (/ (Components|Timeline|GetPlaybackPosition (Variables|Default|GetTimeline_0)) (Variables|Default|GetTotal%20Time)) "World" false) false false))
    (:Finished
      (Variables|Default|SetTotal%20Time 2e+01)
      (Sequencer|Player|Play (Variables|/Script/ActorSequence.ActorSequenceComponent|GetSequencePlayer (Variables|Default|GetFadeToBlack)) :!class /Script/MovieScene.MovieSceneSequencePlayer)
      (Utilities|FlowControl|Delay 1.0)
      (bind _asmy_game_instance (Utilities|Casting|CastToMyGameInstance (Game|GetGameInstance)))
      (bind _output_get (Variables|/Game/Blueprints/MyGameInstance.MyGameInstance_C|SetLevel%20Index _asmy_game_instance (+ (Variables|/Game/Blueprints/MyGameInstance.MyGameInstance_C|GetLevel%20Index _asmy_game_instance) 1)))
      (if (>= _output_get 4)
        (Game|QuitGame 0 "Quit" false)
        (else
          (Game|OpenLevel(byName) (Utilities|Select :Index _output_get :Option%200 "WorkSpace" :Option%201 "Kitchen" :Option%202 "WorkSpace_2" :Option%203 "Cabinet")))))))

(event EventBeginPlay
  (Sequencer|Player|Play (Variables|/Script/ActorSequence.ActorSequenceComponent|GetSequencePlayer (Variables|Default|GetFadeToScene)) :!class /Script/MovieScene.MovieSceneSequencePlayer)
  (Components|Timeline|SetTimelineLength (Variables|Default|GetTimeline_0) (Variables|Default|GetTotal%20Time))
  (bind _outactors (Actor|GetAllActorsOfClass "/Game/Blueprints/BP_Track.BP_Track_C"))
  (Variables|Default|SetBP_Track (Utilities|Array|Get(acopy) _outactors))
  (Timeline|Timeline_0 PlayFromStart
    (:Update
      (Transformation|SetActorLocation (Spline|GetLocationatTime (Variables|/Game/Blueprints/BP_Track.BP_Track_C|GetSpline (Variables|Default|GetBP_Track)) (/ (Components|Timeline|GetPlaybackPosition (Variables|Default|GetTimeline_0)) (Variables|Default|GetTotal%20Time)) "World" false) false false)
      (Transformation|SetWorldRotation (Variables|Default|GetCamera) (Class|SplineComponent|GetRotationatTime (Variables|/Game/Blueprints/BP_Track.BP_Track_C|GetSpline (Variables|Default|GetBP_Track)) (/ (Components|Timeline|GetPlaybackPosition (Variables|Default|GetTimeline_0)) (Variables|Default|GetTotal%20Time)) "World" false) false false))
    (:Finished
      (Variables|Default|SetTotal%20Time 2e+01)
      (Sequencer|Player|Play (Variables|/Script/ActorSequence.ActorSequenceComponent|GetSequencePlayer (Variables|Default|GetFadeToBlack)) :!class /Script/MovieScene.MovieSceneSequencePlayer)
      (Utilities|FlowControl|Delay 1.0)
      (bind _asmy_game_instance (Utilities|Casting|CastToMyGameInstance (Game|GetGameInstance)))
      (bind _output_get (Variables|/Game/Blueprints/MyGameInstance.MyGameInstance_C|SetLevel%20Index _asmy_game_instance (+ (Variables|/Game/Blueprints/MyGameInstance.MyGameInstance_C|GetLevel%20Index _asmy_game_instance) 1)))
      (if (>= _output_get 4)
        (Game|QuitGame 0 "Quit" false)
        (else
          (Game|OpenLevel(byName) (Utilities|Select :Index _output_get :Option%200 "WorkSpace" :Option%201 "Kitchen" :Option%202 "WorkSpace_2" :Option%203 "Cabinet")))))))

(fn ConstructionScript)